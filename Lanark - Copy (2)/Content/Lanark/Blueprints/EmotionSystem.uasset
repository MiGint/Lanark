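; Emotion system Blueprint that models eight compound emotions, such as Love, Awe and Remorse, from four axes: Response, Social, Impulse and Focus.
; Each setter grades one emotion in three intensity tiers when two axes hit exact matching magnitudes, but none is called from live logic here.
; Tick prints the data for debugging, then SetEmotions rebuilds EmotionSystemData from the emotion variables, without passing the axis values through.
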(event EventTick
  (params (DeltaSeconds :type Float%20%28single-precision%29))
  (bind _emotionsystemdata (Variables|Default|GetEmotionSystemData))
  (bind (_response _social _impulse _focus _love _submission _awe _disapproval _remorse _contempt _aggressivness _optimism) (Utilities|Struct|BreakEmotionSystemData _emotionsystemdata))
  (Utilities|FlowControl|Sequence
    (:then_0
      (Development|PrintString (Utilities|String|Append "Remorse: " (Utilities|String|ToString(Integer) _remorse) " " "Contempt: " (Utilities|String|ToString(Integer) _contempt) " " "Aggressivness: " (Utilities|String|ToString(Integer) _aggressivness) " " "Optimism: " (Utilities|String|ToString(Integer) _optimism)) true true "(R=0.000000,G=0.660000,B=1.000000,A=1.000000)" DeltaSeconds))
    (:then_1
      (Development|PrintString (Utilities|String|Append "Response: " (Utilities|String|ToString(Integer) _response) " " "Social: " (Utilities|String|ToString(Integer) _social) " " "Impulse: " (Utilities|String|ToString(Integer) _impulse) " " "Focus: " (Utilities|String|ToString(Integer) _focus) " " "Love: " (Utilities|String|ToString(Integer) _love) " " "Submission: " (Utilities|String|ToString(Integer) _submission) "" "Awe: " (Utilities|String|ToString(Integer) _awe) " " "Disapproval: " (Utilities|String|ToString(Integer) _disapproval)) true true "(R=0.000000,G=0.660000,B=1.000000,A=1.000000)" DeltaSeconds))
    (:then_2
      (CallFunction|SetEmotions))))

(fn ConstructionScript)

(fn SetEmotions
  (Utilities|FlowControl|Sequence
    (:then_8
      (Variables|Default|SetEmotionSystemData (Utilities|Struct|MakeEmotionSystemData 0 0 0 0 (Variables|Default|GetLove) (Variables|Default|GetSubmission) (Variables|Default|GetAwe) (Variables|Default|GetDisapproval) (Variables|Default|GetRemorse) (Variables|Default|GetContempt) (Variables|Default|GetAggressiveness) (Variables|Default|GetOptimism))))))

(fn SetLove
  (bind _emotionsystemdata (Variables|Default|GetEmotionSystemData))
  (bind (_response _social) (Utilities|Struct|BreakEmotionSystemData _emotionsystemdata))
  (if (and (== _response 3) (== _social 3))
    (Variables|Default|SetLove 1)
    (elif (and (== _response 4) (== _social 4))
      (Variables|Default|SetLove 2)
      (elif (and (== _response 5) (== _social 5))
        (Variables|Default|SetLove 3)))))

(fn SetSubmission
  (bind _emotionsystemdata (Variables|Default|GetEmotionSystemData))
  (bind (_response _social _impulse) (Utilities|Struct|BreakEmotionSystemData _emotionsystemdata))
  (if (and (== _social 3) (== _impulse 3))
    (Variables|Default|SetSubmission 1)
    (elif (and (== _social 4) (== _impulse 4))
      (Variables|Default|SetSubmission 2)
      (elif (and (== _social 5) (== _impulse 5))
        (Variables|Default|SetSubmission 3)))))

(fn SetAwe
  (bind _emotionsystemdata (Variables|Default|GetEmotionSystemData))
  (bind (_response _social _impulse _focus) (Utilities|Struct|BreakEmotionSystemData _emotionsystemdata))
  (if (and (== _impulse 3) (== _focus -3))
    (Variables|Default|SetAwe 1)
    (elif (and (== _impulse 4) (== _focus -4))
      (Variables|Default|SetAwe 2)
      (elif (and (== _impulse 5) (== _focus -5))
        (Variables|Default|SetAwe 3)))))

(fn SetDisapproval
  (bind _emotionsystemdata (Variables|Default|GetEmotionSystemData))
  (bind (_response _social _impulse _focus) (Utilities|Struct|BreakEmotionSystemData _emotionsystemdata))
  (if (and (== _response -3) (== _focus -3))
    (Variables|Default|SetDisapproval 1)
    (elif (and (== _response -4) (== _focus -4))
      (Variables|Default|SetDisapproval 2)
      (elif (and (== _response -5) (== _focus -5))
        (Variables|Default|SetDisapproval 3)))))

(fn SetRemorse
  (bind _emotionsystemdata (Variables|Default|GetEmotionSystemData))
  (bind (_response _social) (Utilities|Struct|BreakEmotionSystemData _emotionsystemdata))
  (if (and (== _response -3) (== _social -3))
    (Variables|Default|SetRemorse 1)
    (elif (and (== _response -4) (== _social -4))
      (Variables|Default|SetRemorse 2)
      (elif (and (== _response -5) (== _social -5))
        (Variables|Default|SetRemorse 3)))))

(fn SetContempt
  (bind _emotionsystemdata (Variables|Default|GetEmotionSystemData))
  (bind (_response _social _impulse) (Utilities|Struct|BreakEmotionSystemData _emotionsystemdata))
  (if (and (== _social -3) (== _impulse -3))
    (Variables|Default|SetContempt 1)
    (elif (and (== _social -4) (== _impulse -4))
      (Variables|Default|SetContempt 2)
      (elif (and (== _social -5) (== _impulse -5))
        (Variables|Default|SetContempt 3)))))

(fn SetAggressiveness
  (bind _emotionsystemdata (Variables|Default|GetEmotionSystemData))
  (bind (_response _social _impulse _focus) (Utilities|Struct|BreakEmotionSystemData _emotionsystemdata))
  (if (and (== _impulse -3) (== _focus 3))
    (Variables|Default|SetAggressiveness 1)
    (elif (and (== _impulse -4) (== _focus 4))
      (Variables|Default|SetAggressiveness 2)
      (elif (and (== _impulse -5) (== _focus 5))
        (Variables|Default|SetAggressiveness 3)))))

(fn SetOptimism
  (bind _emotionsystemdata (Variables|Default|GetEmotionSystemData))
  (bind (_response _social _impulse _focus) (Utilities|Struct|BreakEmotionSystemData _emotionsystemdata))
  (if (and (== _response 3) (== _focus 3))
    (Variables|Default|SetOptimism 1)
    (elif (and (== _response 4) (== _focus 4))
      (Variables|Default|SetOptimism 2)
      (elif (and (== _response 5) (== _focus 5))
        (Variables|Default|SetOptimism 3)))))