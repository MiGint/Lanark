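; LoadLevel is a trigger volume actor that streams sublevels in and out as the player character passes through it.
; Overlap begin asynchronously loads LevelToLoad as visible and, if ShouldChangeCharacterPosition is set, moves the player and sets control rotation from PlayerTransform.
; The move starts right after the load request, without waiting for completion.
; Overlap end asynchronously unloads LevelToUnload unless it is None.
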(event OnComponentBeginOverlap(CollisionComponent)
  (params (OverlappedComponent :type Primitive%20Component%20Object%20Reference) (OtherActor :type Actor%20Object%20Reference) (OtherComp :type Primitive%20Component%20Object%20Reference) (OtherBodyIndex :type Integer) (bFromSweep :type Boolean) (SweepResult :type Hit%20Result%20Structure%20%28by%20ref%29))
  (bind _playertransform (Variables|Default|GetPlayerTransform))
  (if (== OtherActor (Game|GetPlayerCharacter 0))
    (Game|LoadStreamLevel(byName) (Variables|Default|GetLevelToLoad) true)
    (if (Variables|Default|GetShouldChangeCharacterPosition)
      (Transformation|SetActorLocation (Game|GetPlayerCharacter 0) (.location _playertransform) false false)
      (Pawn|SetControlRotation (Game|GetPlayerController 0) (.rotation _playertransform)))))

(event OnComponentEndOverlap(CollisionComponent)
  (params (OverlappedComponent :type Primitive%20Component%20Object%20Reference) (OtherActor :type Actor%20Object%20Reference) (OtherComp :type Primitive%20Component%20Object%20Reference) (OtherBodyIndex :type Integer))
  (if (== OtherActor (Game|GetPlayerCharacter 0))
    (if (Utilities|Name|NotEqual(Name) (Variables|Default|GetLevelToUnload) "None")
      (Game|UnloadStreamLevel(byName) (Variables|Default|GetLevelToUnload) false))))

(fn ConstructionScript)