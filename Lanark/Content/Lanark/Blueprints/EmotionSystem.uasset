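; Emotion system actor that derives eight compound emotions, such as Love, Awe and Remorse, from four axes: Response, Social, Impulse and Focus.
; Every Tick it prints the values on screen for debugging, then runs SetEmotions to rebuild the EmotionSystemData struct.
; Each setter grades one emotion 1 to 3 when two axes exactly hit paired thresholds of matching magnitude.
; Unmatched inputs leave the previous level unchanged.
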(event EventTick
  (params (DeltaSeconds :type Float%20%28single-precision%29))
  (bind _emotionsystemdata (Variables|Default|GetEmotionSystemData))
  (bind (_response _social _impulse _focus _love _submission _awe _disapproval _remorse _contempt _aggressivness _optimism) (Utilities|Struct|BreakEmotionSystemData _emotionsystemdata))
  (Utilities|FlowControl|Sequence
    (:then_0
      (Development|PrintString (Utilities|String|Append "Remorse: " (Utilities|String|ToString(Integer) _remorse) " " "Contempt: " (Utilities|String|ToString(Integer) _contempt) " " "Aggressivness: " (Utilities|String|ToString(Integer) _aggressivness) " " "Optimism: " (Utilities|String|ToString(Integer) _optimism)) true true "(R=0.000000,G=0.660000,B=1.000000,A=1.000000)" DeltaSeconds))
    (:then_1
      (Development|PrintString (Utilities|String|Append "Response: " (Utilities|String|ToString(Integer) _response) " " "Social: " (Utilities|String|ToString(Integer) _social) " " "Impulse: " (Utilities|String|ToString(Integer) _impulse) " " "Focus: " (Utilities|String|ToString(Integer) _focus) " " "Love: " (Utilities|String|ToString(Integer) _love) " " "Submission: " (Utilities|String|ToString(Integer) _submission) "" "Awe: " (Utilities|String|ToString(Integer) _awe) " " "Disapproval: " (Utilities|String|ToString(Integer) _disapproval)) true true "(R=0.000000,G=0.660000,B=1.000000,A=1.000000)" DeltaSeconds))
    (:then_2
      (CallFunction|SetEmotions))))

(fn ConstructionScript)

(fn SetEmotions
  (Utilities|FlowControl|Sequence
    (:then_0
      (Utilities|SetLove (.Response (Utilities|Struct|BreakEmotionSystemData (Variables|Default|GetEmotionSystemData))) (.Social (Utilities|Struct|BreakEmotionSystemData (Variables|Default|GetEmotionSystemData)))))
    (:then_1
      (Utilities|SetSubmission (.Impulse (Utilities|Struct|BreakEmotionSystemData (Variables|Default|GetEmotionSystemData))) (.Social (Utilities|Struct|BreakEmotionSystemData (Variables|Default|GetEmotionSystemData)))))
    (:then_2
      (Utilities|SetAwe (.Impulse (Utilities|Struct|BreakEmotionSystemData (Variables|Default|GetEmotionSystemData))) (.Focus (Utilities|Struct|BreakEmotionSystemData (Variables|Default|GetEmotionSystemData)))))
    (:then_3
      (Utilities|SetDisapproval (.Focus (Utilities|Struct|BreakEmotionSystemData (Variables|Default|GetEmotionSystemData))) (.Response (Utilities|Struct|BreakEmotionSystemData (Variables|Default|GetEmotionSystemData)))))
    (:then_4
      (Utilities|SetRemorse (.Response (Utilities|Struct|BreakEmotionSystemData (Variables|Default|GetEmotionSystemData))) (.Social (Utilities|Struct|BreakEmotionSystemData (Variables|Default|GetEmotionSystemData)))))
    (:then_5
      (Utilities|SetContempt (.Impulse (Utilities|Struct|BreakEmotionSystemData (Variables|Default|GetEmotionSystemData))) (.Social (Utilities|Struct|BreakEmotionSystemData (Variables|Default|GetEmotionSystemData)))))
    (:then_6
      (Utilities|SetAggressiveness (.Impulse (Utilities|Struct|BreakEmotionSystemData (Variables|Default|GetEmotionSystemData))) (.Focus (Utilities|Struct|BreakEmotionSystemData (Variables|Default|GetEmotionSystemData)))))
    (:then_7
      (Utilities|SetOptimism (.Focus (Utilities|Struct|BreakEmotionSystemData (Variables|Default|GetEmotionSystemData))) (.Response (Utilities|Struct|BreakEmotionSystemData (Variables|Default|GetEmotionSystemData)))))
    (:then_8
      (Variables|Default|SetEmotionSystemData (Utilities|Struct|MakeEmotionSystemData (.Response (Utilities|Struct|BreakEmotionSystemData (Variables|Default|GetEmotionSystemData))) (.Social (Utilities|Struct|BreakEmotionSystemData (Variables|Default|GetEmotionSystemData))) (.Impulse (Utilities|Struct|BreakEmotionSystemData (Variables|Default|GetEmotionSystemData))) (.Focus (Utilities|Struct|BreakEmotionSystemData (Variables|Default|GetEmotionSystemData))) (Variables|Default|GetLove) (Variables|Default|GetSubmission) (Variables|Default|GetAwe) (Variables|Default|GetDisapproval) (Variables|Default|GetRemorse) (Variables|Default|GetContempt) (Variables|Default|GetAggressiveness) (Variables|Default|GetOptimism))))))