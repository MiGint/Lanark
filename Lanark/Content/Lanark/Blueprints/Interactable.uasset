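; Interactable actor Blueprint that gates player input through its Interactable flag and can be dismissed with a left click.
; Every Tick it disables input on player controller 0 while the flag is true, and enables it otherwise.
; A left mouse press while flagged restores input and destroys the actor.
; BeginPlay stores the actor's starting location in OriginLocation, which these graphs never read.
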(event EventBeginPlay
  (Variables|Default|SetoriginLocation (Transformation|GetActorLocation)))

(event EventTick
  (params (DeltaSeconds :type Float%20%28single-precision%29))
  (bind _returnvalue (Game|GetPlayerController 0))
  (if (Variables|Default|GetInteractable)
    (Input|DisableInput _returnvalue _returnvalue)
    (else
      (Input|EnableInput _returnvalue _returnvalue))))

(event Input|MouseEvents|LeftMouseButton
  (params (Key :type Key%20Structure))
  (bind _returnvalue (Game|GetPlayerController 0))
  (:Pressed
    (if (Variables|Default|GetInteractable)
      (Input|EnableInput _returnvalue _returnvalue)
      (Actor|DestroyActor))))

(fn ConstructionScript)