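; LoadLevel is a trigger volume that streams sublevels in and out as the player character passes through it.
; Beginning overlap loads LevelToLoad asynchronously and makes it visible, while ending overlap unloads LevelToUnload if one is named.
; On exit it can also teleport the player to a configured height at the same X and Y, close a linked Door while setting it openable, and print the positions.
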(event OnComponentBeginOverlap(CollisionComponent)
  (params (OverlappedComponent :type Primitive%20Component%20Object%20Reference) (OtherActor :type Actor%20Object%20Reference) (OtherComp :type Primitive%20Component%20Object%20Reference) (OtherBodyIndex :type Integer) (bFromSweep :type Boolean) (SweepResult :type Hit%20Result%20Structure%20%28by%20ref%29))
  (if (== OtherActor (Game|GetPlayerCharacter 0))
    (Game|LoadStreamLevel(byName) (Variables|Default|GetLevelToLoad) true)))

(event OnComponentEndOverlap(CollisionComponent)
  (params (OverlappedComponent :type Primitive%20Component%20Object%20Reference) (OtherActor :type Actor%20Object%20Reference) (OtherComp :type Primitive%20Component%20Object%20Reference) (OtherBodyIndex :type Integer))
  (bind _returnvalue (Game|GetPlayerCharacter 0))
  (bind _door (Variables|Default|GetDoor))
  (bind _returnvalue_2 (Transformation|GetActorLocation _returnvalue))
  (if (== OtherActor (Game|GetPlayerCharacter 0))
    (Utilities|FlowControl|Sequence
      (:then_0
        (if (Utilities|Name|NotEqual(Name) (Variables|Default|GetLevelToUnload) "None")
          (Game|UnloadStreamLevel(byName) (Variables|Default|GetLevelToUnload) false)))
      (:then_1
        (if (Variables|Default|GetShouldChangeCharacterPosition)
          (Transformation|SetActorLocationAndRotation (Game|GetPlayerCharacter 0) (Math|Vector|MakeVector (.x _returnvalue_2) (.y _returnvalue_2) (+ (.z (Variables|Default|GetPlayerTransform)) (Variables|/Script/Engine.CapsuleComponent|GetCapsuleHalfHeight (Variables|/Script/Engine.Character|GetCapsuleComponent _returnvalue)))) (Transformation|GetActorRotation (Game|GetPlayerController 0)) false true)
          (Default|DoorClose _door)
          (Variables|/Game/Lanark/PreFabs/doors.doors_C|SetcanOpen _door true)
          (Development|PrintString (Utilities|String|Append (Utilities|String|ToString(Vector) (Transformation|GetActorLocation (Game|GetPlayerCharacter 0))) " / " (Utilities|String|ToString(Vector) (Variables|Default|GetPlayerTransform)))))))))

(fn ConstructionScript)